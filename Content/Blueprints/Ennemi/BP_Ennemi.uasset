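; Enemy actor that takes damage, can drop health and awards score when killed.
; SetLife subtracts the given value from Life rather than assigning it.
; At zero or below, it spawns BP_Health roughly half the time, adds a point to the BP_ThirdPersonCharacter player and destroys itself, provided that cast succeeds.
; The event graph is empty, so damage relies on SetLife being called.
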(event EventBeginPlay)

(event Collision|EventActorBeginOverlap
  (params (OtherActor :type Actor%20Object%20Reference)))

(event EventTick
  (params (DeltaSeconds :type Float%20%28single-precision%29)))

(fn ConstructionScript)

(fn SetLife
  (params (Value :type Float%20%28double-precision%29))
  (bind _output_get (Variables|Default|SetLife (- (Variables|Default|GetLife) Value)))
  (if (<= _output_get 0.0)
    (if (<= (Math|Random|RandomInteger 100) 50)
      _
      (else
        (Game|SpawnActorfromClass "/Game/Blueprints/Collectibles/BP_Health.BP_Health_C" (Math|Transform|MakeTransform (Transformation|GetActorLocation) "0, 0, 0" "1.000000,1.000000,1.000000") "Undefined" "MultiplyWithRoot" 0 0)))
    (bind _asbp_third_person_character (Utilities|Casting|CastToBP_ThirdPersonCharacter (Game|GetPlayerCharacter 0)))
    (Default|AddScore _asbp_third_person_character 1)
    (Actor|DestroyActor)))